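; BP_ObCompass is an interactable compass object that shows a prompt widget near the player and can be caught.
; Overlapping the widget collision with BP_ThirdPersonCharacter shows the widget, and leaving hides it.
; Visible and NotVisible events toggle the Lantern component and its children.
; Catched keeps the Lantern visible, disables both colliders and destroys the widget, ending the proximity prompt.
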(event OnComponentBeginOverlap(WId_Coll)
  (params (OverlappedComponent :type Primitive%20Component%20Object%20Reference) (OtherActor :type Actor%20Object%20Reference) (OtherComp :type Primitive%20Component%20Object%20Reference) (OtherBodyIndex :type Integer) (bFromSweep :type Boolean) (SweepResult :type Hit%20Result%20Structure%20%28by%20ref%29))
  (Utilities|Casting|CastToBP_ThirdPersonCharacter OtherActor)
  (Rendering|SetVisibility (Variables|Default|GetWidget) true false))

(event OnComponentEndOverlap(WId_Coll)
  (params (OverlappedComponent :type Primitive%20Component%20Object%20Reference) (OtherActor :type Actor%20Object%20Reference) (OtherComp :type Primitive%20Component%20Object%20Reference) (OtherBodyIndex :type Integer))
  (Utilities|Casting|CastToBP_ThirdPersonCharacter OtherActor)
  (Rendering|SetVisibility (Variables|Default|GetWidget) false false))

(event Custom|NotVisible
  (Rendering|SetVisibility (Variables|Default|GetLantern) false true))

(event Custom|Visible
  (Rendering|SetVisibility (Variables|Default|GetLantern) true true))

(event Custom|Catched
  (Rendering|SetVisibility (Variables|Default|GetLantern) true true)
  (Collision|SetCollisionEnabled (Variables|Default|GetSphere) "NoCollision")
  (Collision|SetCollisionEnabled (Variables|Default|GetWId_Coll) "NoCollision")
  (Components|DestroyComponent (Variables|Default|GetWidget)))

(event EventBeginPlay)

(fn ConstructionScript)