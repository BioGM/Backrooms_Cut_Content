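; BP_L4MP is a lamp actor whose light the player can toggle on and off with the F key while standing within its overlap area.
; Begin and end overlap enable and disable input for player controller 0, without checking which actor overlapped.
; Each F press flips the Switch flag and sets the LampLight intensity to either zero or a fixed bright value.
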(event EventBeginPlay)

(event Collision|EventActorBeginOverlap
  (params (OtherActor :type Actor%20Object%20Reference))
  (Input|EnableInput (Game|GetPlayerController 0)))

(event EventTick
  (params (DeltaSeconds :type Float%20%28single-precision%29)))

(event Collision|EventActorEndOverlap
  (params (OtherActor :type Actor%20Object%20Reference))
  (Input|DisableInput (Game|GetPlayerController 0)))

(event Input|KeyboardEvents|F
  (params (Key :type Key%20Structure :default "None"))
  (bind _lamplight (Variables|Default|GetLampLight))
  (:Pressed
    (if (Variables|Default|GetSwitch)
      (Variables|Default|SetSwitch false)
      (Rendering|Components|Light|SetIntensity _lamplight 0.0)
      (else
        (Variables|Default|SetSwitch true)
        (Rendering|Components|Light|SetIntensity _lamplight 5e+03)))))

(fn ConstructionScript)