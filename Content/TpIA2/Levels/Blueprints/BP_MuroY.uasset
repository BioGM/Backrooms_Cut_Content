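; BP_MuroY is a wall actor that moves vertically when the third-person character enters its trigger box.
; Box overlap caches the Pared component's location and plays a Timeline that drives its world Z from a fixed 125-unit base, keeping X and Y.
; When the character leaves, the Timeline reverses after a ten-second delay.
; Height-check branches and a second delay are left unconnected.
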(event OnComponentEndOverlap(Box)
  (params (OverlappedComponent :type Primitive%20Component%20Object%20Reference) (OtherActor :type Actor%20Object%20Reference) (OtherComp :type Primitive%20Component%20Object%20Reference) (OtherBodyIndex :type Integer))
  (bind _vecpos (Variables|Default|GetVecPos))
  (Utilities|Casting|CastToBP_ThirdPersonCharacter OtherActor)
  (Utilities|FlowControl|Delay 1e+01)
  (bind _newtrack_0 (Timeline|Timeline Reverse)
    (:Update
      (Transformation|SetWorldLocation (Variables|Default|GetPared) (Math|Vector|MakeVector (.x _vecpos) (.y _vecpos) (+ _newtrack_0 125.0)) false false))))

(event OnComponentBeginOverlap(Box)
  (params (OverlappedComponent :type Primitive%20Component%20Object%20Reference) (OtherActor :type Actor%20Object%20Reference) (OtherComp :type Primitive%20Component%20Object%20Reference) (OtherBodyIndex :type Integer) (bFromSweep :type Boolean) (SweepResult :type Hit%20Result%20Structure%20%28by%20ref%29))
  (Utilities|Casting|CastToBP_ThirdPersonCharacter OtherActor)
  (Variables|Default|SetVecPos (Transformation|GetWorldLocation (Variables|Default|GetPared)))
  (bind _newtrack_0 (Timeline|Timeline PlayFromStart)
    (:Update
      (Transformation|SetWorldLocation (Variables|Default|GetPared) (Math|Vector|MakeVector (.x (Variables|Default|GetVecPos)) (.y (Variables|Default|GetVecPos)) (+ _newtrack_0 125.0)) false false))))

(event Collision|EventActorBeginOverlap
  (params (OtherActor :type Actor%20Object%20Reference)))

(event EventTick
  (params (DeltaSeconds :type Float%20%28single-precision%29)))

(event EventBeginPlay)

(fn ConstructionScript)