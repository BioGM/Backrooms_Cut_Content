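; BP_DoorsD is a level puzzle actor that repositions two doors, DoorAa and DoorBb, according to two boolean flags.
; Two trigger boxes respond to BP_ThirdPersonCharacter: BoxColl clears DoorA and toggles DoorB, while BoxColl1 sets DoorA and clears DoorB.
; Any overlap with the actor reads those flags and snaps the doors to hardcoded relative locations without animation, moving both or only DoorBb depending on the combination.
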(event OnComponentBeginOverlap(BoxColl)
  (params (OverlappedComponent :type Primitive%20Component%20Object%20Reference) (OtherActor :type Actor%20Object%20Reference) (OtherComp :type Primitive%20Component%20Object%20Reference) (OtherBodyIndex :type Integer) (bFromSweep :type Boolean) (SweepResult :type Hit%20Result%20Structure%20%28by%20ref%29))
  (Utilities|Casting|CastToBP_ThirdPersonCharacter OtherActor)
  (Variables|Default|SetDoorA false)
  (if (Variables|Default|GetDoorB)
    (Variables|Default|SetDoorB false)
    (else
      (Variables|Default|SetDoorB true))))

(event OnComponentBeginOverlap(BoxColl1)
  (params (OverlappedComponent :type Primitive%20Component%20Object%20Reference) (OtherActor :type Actor%20Object%20Reference) (OtherComp :type Primitive%20Component%20Object%20Reference) (OtherBodyIndex :type Integer) (bFromSweep :type Boolean) (SweepResult :type Hit%20Result%20Structure%20%28by%20ref%29))
  (Utilities|Casting|CastToBP_ThirdPersonCharacter OtherActor)
  (Variables|Default|SetDoorA true)
  (Variables|Default|SetDoorB false))

(event EventBeginPlay)

(event Collision|EventActorBeginOverlap
  (params (OtherActor :type Actor%20Object%20Reference))
  (bind _doorb (Variables|Default|GetDoorB))
  (if (Variables|Default|GetDoorA)
    (if (not _doorb)
      (Transformation|SetRelativeTransform (Variables|Default|GetDoor_Aa) (Math|Transform|MakeTransform "-720.000000,368.000000,0.000000" "0, 0, 0" (Variables|/Script/Engine.SceneComponent|GetRelativeScale3D (Variables|Default|GetDoor_Aa))) false false)
      (Transformation|SetRelativeTransform (Variables|Default|GetDoor_Bb) (Math|Transform|MakeTransform "280.000000,-650.000000,0.000000" "0, 0, 0" (Variables|/Script/Engine.SceneComponent|GetRelativeScale3D (Variables|Default|GetDoor_Bb))) false false))
    (elif _doorb
      (Transformation|SetRelativeTransform (Variables|Default|GetDoor_Aa) (Math|Transform|MakeTransform "-520.000000,368.000000,0.000000" "0, 0, 0" (Variables|/Script/Engine.SceneComponent|GetRelativeScale3D (Variables|Default|GetDoor_Aa))) false false)
      (Transformation|SetRelativeTransform (Variables|Default|GetDoor_Bb) (Math|Transform|MakeTransform "480.000000,-650.000000,0.000000" "0, 0, 0" (Variables|/Script/Engine.SceneComponent|GetRelativeScale3D (Variables|Default|GetDoor_Bb))) false false)
      (else
        (Transformation|SetRelativeTransform (Variables|Default|GetDoor_Bb) (Math|Transform|MakeTransform "280.000000,-650.000000,0.000000" "0, 0, 0" (Variables|/Script/Engine.SceneComponent|GetRelativeScale3D (Variables|Default|GetDoor_Bb))) false false)))))

(event EventTick
  (params (DeltaSeconds :type Float%20%28single-precision%29)))

(fn ConstructionScript)