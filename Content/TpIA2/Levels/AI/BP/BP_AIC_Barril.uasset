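; AI controller for the barrel (Barril) enemy that runs the BT_Barril behavior tree on possession.
; Hearing stimuli from AI perception write their location to the SoundLocation blackboard key.
; OnRange? sets HasOnRange according to whether the player is within 200 units of a given position.
; MoveToPlayer is an empty stub, and the debug line drawing is disconnected.
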(event OnTargetPerceptionUpdated(AIPerception)
  (params (Actor :type Actor%20Object%20Reference) (Stimulus :type AI%20Stimulus%20Structure))
  (bind _returnvalue (Class|AIPerceptionSystem|GetSenseClassforStimulus Stimulus))
  (if (== _returnvalue "/Script/AIModule.AISense_Hearing")
    (AI|Components|Blackboard|SetValueasVector (Variables|Default|GetBlackboard) (Variables|Default|GetSoundLocation) (.StimulusLocation (Utilities|Struct|BreakAIStimulus Stimulus)))))

(event EventBeginPlay)

(event EventTick
  (params (DeltaSeconds :type Float%20%28single-precision%29)))

(event EventPossess
  (params (PossessedPawn :type Pawn%20Object%20Reference))
  (AI|RunBehaviorTree "/Game/TpIA2/Levels/AI/BT_Barril.BT_Barril"))

(fn ConstructionScript)

(fn MovetoPlayer)

(fn OnRange?
  (params (Position :type Vector))
  (bind _blackboard (Variables|Default|GetBlackboard))
  (bind _hasonrange (Variables|Default|GetHasOnRange))
  (bind _asbp_third_person_character (Utilities|Casting|CastToBP_ThirdPersonCharacter (Game|GetPlayerCharacter 0)))
  (if (< (Math|Vector|VectorLength (- (Transformation|GetActorLocation _asbp_third_person_character) Position)) 2e+02)
    (AI|Components|Blackboard|SetValueasBool _blackboard _hasonrange true)
    (return false)
    (else
      (AI|Components|Blackboard|SetValueasBool _blackboard _hasonrange (< (Math|Vector|VectorLength (- (Transformation|GetActorLocation _asbp_third_person_character) Position)) 2e+02)))))